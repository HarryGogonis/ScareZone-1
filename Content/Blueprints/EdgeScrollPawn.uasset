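; Camera pawn that pans horizontally using movement input plus edge-scroll axis offsets, which are read but not set here.
; Each axis event moves the actor along the camera's yaw-only forward or right vector, scaled by movement speed.
; On construction, UpdateCameraLocation places the camera using PointOnASphere with radius and two angles, then aims it at the pawn's local origin.
; The spherical math in PointOnASphere appears unconnected.
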(event Input|AxisEvents|InputAxisMoveRight
  (params (AxisValue :type Float%20%28single-precision%29))
  ;[1 1 1] Movement
  (Transformation|SetActorLocation (+ (* (Math|Vector|GetRightVector (Math|Rotator|MakeRotator 0.0 0.0 (.yaw (Transformation|GetWorldRotation (Variables|Default|GetCamera))))) (* (+ AxisValue (Variables|Default|GetEdgeRightAxis)) (Variables|Default|GetMovementSpeed))) (Transformation|GetActorLocation)) false false))

(event Input|AxisEvents|InputAxisMoveForward
  (params (AxisValue :type Float%20%28single-precision%29))
  ;[1 1 1] Movement
  (Transformation|SetActorLocation (+ (Transformation|GetActorLocation) (* (Math|Vector|GetForwardVector (Math|Rotator|MakeRotator 0.0 0.0 (.yaw (Transformation|GetWorldRotation (Variables|Default|GetCamera))))) (* (+ AxisValue (Variables|Default|GetEdgeForwardAxis)) (Variables|Default|GetMovementSpeed)))) false false))

(fn ConstructionScript
  (CallFunction|UpdateCameraLocation))

(fn UpdateCameraLocation
  (Transformation|SetRelativeLocation (Variables|Default|GetCamera) (.Location (Utilities|PointonASphere (Variables|Default|GetCameraRadius) (Variables|Default|GetCameraZAngle) (Variables|Default|GetCameraHeightAngle))) false false)
  (Transformation|SetRelativeRotation (Variables|Default|GetCamera) (Math|Rotator|FindLookatRotation (Variables|/Script/Engine.SceneComponent|GetRelativeLocation (Variables|Default|GetCamera)) (Math|Vector|MakeVector 0.0 0.0 0.0)) false false)
  (return))